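; Player-controlled boat that moves by physics forces, with mouse-driven camera look.
; Forward/back and right/left axes push the static mesh along the actor's own forward and right vectors as mass-independent acceleration.
; Each tick the actor's yaw eases toward its velocity direction by a fixed lerp alpha, keeping pitch and roll.
; Mouse axes feed controller yaw and pitch, scaled by delta time.
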(event `InputAxisKey|MouseX`
  (params (AxisValue :type "Float (single-precision)")))

(event `InputAxisKey|MouseX`
  (params (AxisValue :type "Float (single-precision)"))
  ;[1 1 1] Camera Control
  (`self.Look Left/Right` AxisValue))

(event `InputAxisKey|MouseY`
  (params (AxisValue :type "Float (single-precision)"))
  ;[1 1 1] Camera Control
  (`self.Look Up/Down` AxisValue))

(event `self.ReceiveTick`
  (params (DeltaSeconds :type "Float (single-precision)"))
  (bind _returnvalue (`self.K2_GetActorRotation`))
  (bind (_returnvalue_roll _returnvalue_pitch _returnvalue_yaw) (`KismetMathLibrary.BreakRotator` (`KismetMathLibrary.RLerp` _returnvalue (`KismetMathLibrary.Conv_VectorToRotator` (`self.GetVelocity`)) 0.1 true)))
  ;[1 1 1] Rotation
  (`self.K2_SetActorRotation` (`KismetMathLibrary.MakeRotator` (.roll _returnvalue) (.pitch _returnvalue) _returnvalue_yaw)))

(event `InputAxis|Move Forward / Backward`
  (params (AxisValue :type "Float (single-precision)"))
  ;[1 1 1] Allows boat to move forward and backward
  (`self.Add Movement Force` AxisValue (`self.GetActorForwardVector`)))

(event `InputAxis|Move Right / Left`
  (params (AxisValue :type "Float (single-precision)"))
  ;[1 1 1] Allows boat to move left and right
  (`self.Add Movement Force` AxisValue (`self.GetActorRightVector`)))

(fn `Look Left/Right`
  (params (A :type "Float (double-precision)"))
  (`self.AddControllerYawInput` (* A (`GameplayStatics.GetWorldDeltaSeconds`) 80.0)))

(fn `Look Up/Down`
  (params (A :type "Float (double-precision)"))
  (`self.AddControllerPitchInput` (* A (`GameplayStatics.GetWorldDeltaSeconds`) 80.0)))

(fn `UserConstructionScript`)