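; VehicleMovement drives the Ship actor it finds at BeginPlay, turning player axis input into boat movement.
; Both axes call AddMovementForce, which pushes the ship's static mesh with a speed-scaled acceleration.
; Forward/backward uses the ship's right vector, while right/left keeps only the negated Z of its forward vector.
; Each tick eases yaw toward the velocity direction at a fixed lerp alpha, preserving pitch and roll.
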(event `self.ReceiveBeginPlay`
  (bind _returnvalue (`GameplayStatics.GetActorOfClass` "/Game/Blueprints/Boat/Ship.Ship_C"))
  (set `self.Target` _returnvalue))

(event `self.ReceiveTick`
  (params (DeltaSeconds :type "Float (single-precision)"))
  (bind _returnvalue (`Actor.K2_GetActorRotation` (`self.Target`)))
  (bind (_returnvalue_roll _returnvalue_pitch _returnvalue_yaw) (`KismetMathLibrary.BreakRotator` (`KismetMathLibrary.RLerp` _returnvalue (`KismetMathLibrary.Conv_VectorToRotator` (`Actor.GetVelocity` (`self.Target`))) 0.1 true)))
  (`Actor.K2_SetActorRotation` (`self.Target`) (`KismetMathLibrary.MakeRotator` (.roll _returnvalue) (.pitch _returnvalue) _returnvalue_yaw) false))

(event `InputAxis|Move Forward / Backward`
  (params (AxisValue :type "Float (single-precision)"))
  ;[1 1 1] Allows boat to move forward and backward
  (`self.AddMovementForce` AxisValue (`Actor.GetActorRightVector` (`self.Target`)) (`self.Target`)))

(event `InputAxis|Move Right / Left`
  (params (AxisValue :type "Float (single-precision)"))
  ;[1 1 1] Allows boat to move left and right
  (`self.AddMovementForce` AxisValue (* (`Actor.GetActorForwardVector` (`self.Target`)) (0.0 0.0 -1.0)) (`self.Target`)))