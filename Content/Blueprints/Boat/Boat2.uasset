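; Drivable boat pawn that the player can board from a trigger box and leave by pressing E.
; Overlapping the box prints a prompt and binds the third-person character's Interact dispatcher to possess the boat, storing that character as driver for re-possession on exit.
; Movement axes push the static mesh with acceleration-based physics forces along forward and right vectors, while Tick smoothly turns yaw toward the velocity direction.
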(event `self.ReceiveTick`
  (params (DeltaSeconds :type "Float (single-precision)"))
  (bind _returnvalue (`self.K2_GetActorRotation`))
  (bind (_returnvalue_roll _returnvalue_pitch _returnvalue_yaw) (`KismetMathLibrary.BreakRotator` (`KismetMathLibrary.RLerp` _returnvalue (`KismetMathLibrary.Conv_VectorToRotator` (`self.GetVelocity`)) 0.1 true)))
  (`self.K2_SetActorRotation` (`KismetMathLibrary.MakeRotator` (.roll _returnvalue) (.pitch _returnvalue) _returnvalue_yaw)))

(event `self.ReceiveBeginPlay`
  (set `self.Boat Pawn` self))

(event `InputAxis|Move Forward / Backward`
  (params (AxisValue :type "Float (single-precision)"))
  ;[1 1 1] Allows boat to move forward and backward
  (`self.Add Movement Force` AxisValue (`self.GetActorForwardVector`)))

(event `InputAxis|Move Right / Left`
  (params (AxisValue :type "Float (single-precision)"))
  ;[1 1 1] Allows boat to move left and right
  (`self.Add Movement Force` AxisValue (`self.GetActorRightVector`)))

(event `self.PossesionBox.OnComponentBeginOverlap`
  (params (OverlappedComponent :type "PrimitiveComponent Object Reference") (OtherActor :type "Actor Object Reference") (OtherComp :type "PrimitiveComponent Object Reference") (OtherBodyIndex :type Integer) (bFromSweep :type Boolean) (SweepResult :type "HitResult Structure (by ref)"))
  (`KismetSystemLibrary.PrintText` "Press E To Enter the Vehicle")
  (bind _asbp_third_person_character (cast `/Game/ThirdPerson/Blueprints/BP_ThirdPersonCharacter` OtherActor))
  (add `/Game/ThirdPerson/Blueprints/BP_ThirdPersonCharacter.Interact` _asbp_third_person_character (delegate `TakeControlOfCar`)))

(event `self.PossesionBox.OnComponentEndOverlap`
  (params (OverlappedComponent :type "PrimitiveComponent Object Reference") (OtherActor :type "Actor Object Reference") (OtherComp :type "PrimitiveComponent Object Reference") (OtherBodyIndex :type Integer))
  (bind _asbp_third_person_character (cast `/Game/ThirdPerson/Blueprints/BP_ThirdPersonCharacter` OtherActor))
  (clear `/Game/ThirdPerson/Blueprints/BP_ThirdPersonCharacter.Interact` _asbp_third_person_character))

(event `TakeControlOfCar`
  (set `self.Driver` (`GameplayStatics.GetPlayerCharacter` 0))
  (`Controller.Possess` (`GameplayStatics.GetPlayerController` 0) self))

(event `Key|E`
  (params (Key :type "Key Structure"))
  (:`Pressed`
    (`Controller.Possess` (`GameplayStatics.GetPlayerController` 0) (`self.Driver`))))

(fn `UserConstructionScript`)