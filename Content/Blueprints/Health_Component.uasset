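; Health component that tracks its owner's current health and death state.
; On BeginPlay it binds to the owner's OnTakeAnyDamage and passes damage as a negative change to AdjustHealth.
; AdjustHealth clamps health between zero and MaxHealth and calls Death at zero, which sets IsDead and prints debug text.
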(event `self.ReceiveBeginPlay`
  (add `Actor.OnTakeAnyDamage` (`self.GetOwner`) (delegate `OnDamageTaken`)))

(event `OnDamageTaken`
  (params (DamagedActor :type "Actor Object Reference") (Damage :type "Float (single-precision)") (DamageType :type "DamageType Object Reference") (InstigatedBy :type "Controller Object Reference") (DamageCauser :type "Actor Object Reference"))
  (`self.AdjustHealth` (* Damage -1.0))
  (`KismetSystemLibrary.PrintString` (`KismetStringLibrary.Conv_DoubleToString` (`self.CurrentHealth`))))

(event `AdjustHealth`
  (params (`Health Added` :type "Float (double-precision)"))
  (set `self.CurrentHealth` (`KismetMathLibrary.FClamp` (+ (`self.CurrentHealth`) `Health Added`) 0.0 (`self.MaxHealth`)))
  (if (<= (`self.CurrentHealth`) 0.0)
    (`self.Death`)))

(event `Death`
  (set `self.IsDead` true)
  (`KismetSystemLibrary.PrintString` "You Dead"))