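; HoverRide is a possessable boat-style vehicle Blueprint whose graph handles engine audio.
; On player possession it plays a start sound, then after a delay activates the motor cue and drives its volume through a timeline.
; If IsIn is set when that finishes, a gate opens so Tick maps the hull's physics speed to the cue's Pitch and Volume parameters.
; Unpossession mutes the cue but leaves the gate open.
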(event `self.ReceivePossessed`
  (params (NewController :type "Controller Object Reference"))
  (bind _motorboat_bass_cue (`self.MotorBoat_Bass_Cue`))
  (bind _motorboat_bass_cue_2 (`self.MotorBoat_Bass_Cue`))
  (bind _newvar_0_0 (`self.NewVar_0_0`))
  ;[1 1 1] Start Sound
  (if (`Controller.IsPlayerController` NewController)
    (`GameplayStatics.PlaySoundAtLocation` null (`SceneComponent.K2_GetComponentLocation` (`self.Boat_Exterior`)) (struct) 1.0 1.0 0.0 null null null null)
    (`KismetSystemLibrary.Delay` 1.0)
    (`ActorComponent.Activate` _motorboat_bass_cue false)
    (bind (_direction _volume) (`Timeline|Sound`)
      (:`Update`
        (`AudioComponent.SetVolumeMultiplier` _motorboat_bass_cue _volume))
      (:`Finished`
        (if (`self.IsIn`)
          (`AudioComponent.SetVolumeMultiplier` _motorboat_bass_cue 2.0)
          (goto _label :!via `Open`)
          (else
            (`AudioComponent.SetVolumeMultiplier` _motorboat_bass_cue 0.0)))))))

(event `self.ReceiveUnpossessed`
  (params (OldController :type "Controller Object Reference"))
  ;[1 1 1] Stop Playing Sound when Exited
  (if (`Controller.IsPlayerController` OldController)
    (`AudioComponent.SetVolumeMultiplier` (`self.MotorBoat_Bass_Cue`) 0.0)))

(event `self.ReceiveTick`
  (params (DeltaSeconds :type "Float (single-precision)"))
  (bind _motorboat_bass_cue (`self.MotorBoat_Bass_Cue`))
  (bind _newvar_0_0 (`self.NewVar_0_0`))
  (`parent.ReceiveTick` DeltaSeconds)
  ;[1 1 1] Boat Sound
  (`/Engine/EditorBlueprintResources/StandardMacros.Gate` true :!label _label
    (:`Exit`
      (bind _returnvalue (`PrimitiveComponent.GetPhysicsLinearVelocity` (`self.Boat_Exterior`) "None"))
      (set `self.NewVar_0_0` (`KismetMathLibrary.MapRangeClamped` (/ (`KismetMathLibrary.VSize` _returnvalue) 1.0) 70.0 2000.0 0.0 100.0))
      (`AudioComponent.SetFloatParameter` _motorboat_bass_cue "Pitch" _newvar_0_0)
      (`AudioComponent.SetFloatParameter` _motorboat_bass_cue "Volume" _newvar_0_0))))

(fn `UserConstructionScript`
  (`parent.UserConstructionScript`))