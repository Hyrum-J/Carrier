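; PowerBoat is a drivable motorboat Blueprint that adds engine audio, splash effects and propeller and rudder animation.
; Player possession plays a start sound, fades in motor volume through a timeline, then opens a gate; unpossession mutes the motor.
; While occupied, Tick spins the rotor by power, angles the rudder by turn rate, and feeds that gate, where hull velocity drives sound parameters and splash material opacity.
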(event `self.ReceiveBeginPlay`
  (bind _splash (`self.Splash`))
  ;[1 1 1] Dynamic Material for splash
  (`parent.ReceiveBeginPlay`)
  (bind _returnvalue (`PrimitiveComponent.CreateDynamicMaterialInstance` _splash 0 null "None"))
  (set `self.Mat_0` _returnvalue)
  (bind _returnvalue_2 (`PrimitiveComponent.CreateDynamicMaterialInstance` _splash 1 null "None"))
  (set `self.Mat_1` _returnvalue_2))

(event `self.ReceivePossessed`
  (params (NewController :type "Controller Object Reference"))
  (bind _motorboat_mixed (`self.MotorBoat_Mixed`))
  (bind _motorboat_mixed_2 (`self.MotorBoat_Mixed`))
  (bind _newvar_0_0 (`self.NewVar_0_0`))
  ;[1 1 1] Start Sound
  (if (`Controller.IsPlayerController` NewController)
    (`GameplayStatics.PlaySoundAtLocation` null (`SceneComponent.K2_GetComponentLocation` (`self.Boat_Exterior`)) (struct) 3.0 1.0 0.0 null null null null)
    (`KismetSystemLibrary.Delay` 1.0)
    (bind (_direction _volume) (`Timeline|Timeline_0`)
      (:`Update`
        (`AudioComponent.SetVolumeMultiplier` _motorboat_mixed_2 _volume))
      (:`Finished`
        (if (`self.IsIn`)
          (`AudioComponent.SetVolumeMultiplier` _motorboat_mixed_2 2.0)
          (goto _label :!via `Open`)
          (else
            (`AudioComponent.SetVolumeMultiplier` _motorboat_mixed_2 0.0)))))))

(event `self.ReceiveUnpossessed`
  (params (OldController :type "Controller Object Reference"))
  ;[1 1 1] Stop Playing Sound when Exited
  (if (`Controller.IsPlayerController` OldController)
    (`AudioComponent.SetVolumeMultiplier` (`self.MotorBoat_Mixed`) 0.0)))

(event `self.ReceiveTick`
  (params (DeltaSeconds :type "Float (single-precision)"))
  (bind _motorboat_mixed (`self.MotorBoat_Mixed`))
  (bind _newvar_0_0 (`self.NewVar_0_0`))
  (`parent.ReceiveTick` DeltaSeconds)
  ;[1 1 1] Defines Rotation of the blades accoring to the speed of the boat
  (if (`self.IsIn`)
    (set `self.Rotation` (+ (`self.Rotation`) (+ (* (`KismetMathLibrary.Abs` (`self.Power`)) 25.0) 6.0)))
    (`SceneComponent.K2_SetRelativeRotation` (`self.Rotor`) (`KismetMathLibrary.MakeRotator` (mod (`self.Rotation`) 360.0) 0.0 180.0) false false)
    ;[1 1 1] Rotation of the rudurs while taking a turn
    (`SceneComponent.K2_SetRelativeRotation` (`self.Rudur`) (`KismetMathLibrary.MakeRotator` 0.0 0.0 (- (* (/ (`self.Power`) (`KismetMathLibrary.Abs` (`self.Power`))) (* (`self.TurnRate`) -20.0)) 90.0)) false false)
    ;[1 1 1] Boat Sound
    (`/Engine/EditorBlueprintResources/StandardMacros.Gate` true :!label _label
      (:`Exit`
        (bind _returnvalue (`PrimitiveComponent.GetPhysicsLinearVelocity` (`self.Boat_Exterior`) "None"))
        (bind _returnvalue_2 (`KismetMathLibrary.VSize` _returnvalue))
        (set `self.NewVar_0_0` (`KismetMathLibrary.MapRangeClamped` (/ _returnvalue_2 1.0) 70.0 3750.0 0.0 200.0))
        (`AudioComponent.SetFloatParameter` _motorboat_mixed "Pitch" _newvar_0_0)
        (`AudioComponent.SetFloatParameter` _motorboat_mixed "Volume" _newvar_0_0)
        (`AudioComponent.SetFloatParameter` _motorboat_mixed "CrossFade" _newvar_0_0)
        ;[1 1 1] ParitcleSystemOpacity
        (`MaterialInstanceDynamic.SetScalarParameterValue` (`self.Mat_0`) "Opacity" (`KismetMathLibrary.MapRangeClamped` _returnvalue_2 550.0 1200.0 0.0 1.0))
        (`MaterialInstanceDynamic.SetScalarParameterValue` (`self.Mat_1`) "Opacity" (`KismetMathLibrary.MapRangeClamped` _returnvalue_2 350.0 800.0 0.5 1.0))))))

(fn `UserConstructionScript`
  (`parent.UserConstructionScript`))