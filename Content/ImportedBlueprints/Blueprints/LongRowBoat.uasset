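; Possessable long rowboat that animates its two oars and adds speed-driven splash and water sound.
; Possession starts the oar animations (looping for a player controller), a player leaving stops them, and a RowAnimation event sets their play rate.
; Tick derives a dead-zoned, clamped value from the hull's forward physics velocity to drive water volume and the opacity of one dynamic material shared across the splash meshes.
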(event `self.ReceiveBeginPlay`
  ;[1 1 1] Begin Play
  (`parent.ReceiveBeginPlay`)
  (`SkeletalMeshComponent.SetPosition` (`self.Row_R`) 2.5 true)
  (`SkeletalMeshComponent.SetPosition` (`self.Row_L`) 2.5 true)
  (bind _returnvalue (`PrimitiveComponent.CreateDynamicMaterialInstance` (`self.SplashSmall`) 0 null "None"))
  (set `self.Mat_0` _returnvalue)
  (`PrimitiveComponent.SetMaterial` (`self.SplashSmall1`) 0 (`self.Mat_0`))
  (`PrimitiveComponent.SetMaterial` (`self.SplashSmall2`) 0 (`self.Mat_0`))
  (`PrimitiveComponent.SetMaterial` (`self.SplashSmall3`) 0 (`self.Mat_0`))
  (`PrimitiveComponent.SetMaterial` (`self.SplashSmall4`) 0 (`self.Mat_0`))
  (`PrimitiveComponent.SetMaterial` (`self.SplashSmall5`) 0 (`self.Mat_0`))
  (`PrimitiveComponent.SetMaterial` (`self.SplashSmall7`) 0 (`self.Mat_0`))
  (`PrimitiveComponent.SetMaterial` (`self.SplashSmall6`) 0 (`self.Mat_0`)))

(event `self.ReceivePossessed`
  (params (NewController :type "Controller Object Reference"))
  ;[1 1 1] Start Playing The Row Animation
  (`SkeletalMeshComponent.Play` (`self.Row_R`) (`Controller.IsPlayerController` NewController))
  (`SkeletalMeshComponent.Play` (`self.Row_L`) (`Controller.IsPlayerController` NewController)))

(event `self.ReceiveUnpossessed`
  (params (OldController :type "Controller Object Reference"))
  ;[1 1 1] Stop playing animation
  (if (`Controller.IsPlayerController` OldController)
    (`SkeletalMeshComponent.Stop` (`self.Row_R`))
    (`SkeletalMeshComponent.Stop` (`self.Row_L`))))

(event `self.ReceiveTick`
  (params (DeltaSeconds :type "Float (single-precision)"))
  (`parent.ReceiveTick` DeltaSeconds)
  ;[1 1 1] Find Forward Velocity and Determine the play rate of the Row Animation
  (bind _returnvalue (`PrimitiveComponent.GetPhysicsLinearVelocity` (`self.Boat_Exterior`) "None"))
  (bind _returnvalue_2 (* (/ (`KismetMathLibrary.VSize` _returnvalue) 85000.0) (`KismetMathLibrary.Dot_VectorVector` _returnvalue (`KismetMathLibrary.GetForwardVector` (`SceneComponent.K2_GetComponentRotation` (`self.Boat_Exterior`))))))
  (bind _returnvalue_3 (`KismetMathLibrary.Abs` (`KismetMathLibrary.SelectFloat` _returnvalue_2 0.0 (or (> _returnvalue_2 0.04) (< _returnvalue_2 -0.04)))))
  (`AudioComponent.SetVolumeMultiplier` (`self.Water_Boat_Cue`) (`KismetMathLibrary.FClamp` (/ _returnvalue_3 10.0) 0.05 0.2))
  (`MaterialInstanceDynamic.SetScalarParameterValue` (`self.Mat_0`) "Opacity" (`KismetMathLibrary.FClamp` _returnvalue_3 0.1)))

(event `self.RowAnimation`
  (params (RowSpeed :type "Float (double-precision)"))
  ;[1 1 1] Row Animation
  (`SkeletalMeshComponent.SetPlayRate` (`self.Row_R`) (* RowSpeed 2.0))
  (`SkeletalMeshComponent.SetPlayRate` (`self.Row_L`) (* RowSpeed 2.0)))

(fn `UserConstructionScript`
  (`parent.UserConstructionScript`))