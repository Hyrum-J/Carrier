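; Ship Blueprint that animates a boat's rotors and rudder, with BeginPlay and construction deferring to the parent class.
; Each Tick while IsIn is set, both rotors roll by an accumulated angle that grows with the magnitude of Power, plus a constant idle spin.
; The rudder's yaw follows TurnRate, flipped by the sign of Power, around a fixed offset.
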(event `self.ReceiveBeginPlay`
  (`parent.ReceiveBeginPlay`))

(event `self.ReceiveTick`
  (params (DeltaSeconds :type "Float (single-precision)"))
  (`parent.ReceiveTick` DeltaSeconds)
  ;[1 1 1] Defines Rotation of the blades accoring to the speed of the boat
  (if (`self.IsIn`)
    (set `self.Rotation` (+ (`self.Rotation`) (+ (* (`KismetMathLibrary.Abs` (`self.Power`)) 25.0) 6.0)))
    (`SceneComponent.K2_SetRelativeRotation` (`self.Rotor`) (`KismetMathLibrary.MakeRotator` (mod (`self.Rotation`) 360.0)) false false)
    (`SceneComponent.K2_SetRelativeRotation` (`self.Rotor1`) (`KismetMathLibrary.MakeRotator` (mod (`self.Rotation`) 360.0)) false false)
    ;[1 1 1] Rotation of the rudurs while taking a turn
    (`SceneComponent.K2_SetRelativeRotation` (`self.Rudur`) (`KismetMathLibrary.MakeRotator` 0.0 0.0 (- (* (/ (`self.Power`) (`KismetMathLibrary.Abs` (`self.Power`))) (* (`self.TurnRate`) -20.0)) 90.0)) false false)))

(fn `UserConstructionScript`
  (`parent.UserConstructionScript`))