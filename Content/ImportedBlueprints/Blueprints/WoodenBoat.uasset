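; WoodenBoat is a possessable rowing boat Blueprint that animates its left and right rows.
; Possession plays RowR and RowL, passing whether the new controller is a player controller as the Play argument, and losing a player controller stops both.
; A RowAnimation event scales the incoming row speed to set both play rates.
; BeginPlay, Tick and construction only call the parent, and the overlap event is disabled.
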(event `self.ReceiveBeginPlay`
  (`parent.ReceiveBeginPlay`))

(event `self.ReceivePossessed`
  (params (NewController :type "Controller Object Reference"))
  ;[1 1 1] Start Playing The Row Animation
  (`SkeletalMeshComponent.Play` (`self.Row_R`) (`Controller.IsPlayerController` NewController))
  (`SkeletalMeshComponent.Play` (`self.Row_L`) (`Controller.IsPlayerController` NewController)))

(event `self.ReceiveUnpossessed`
  (params (OldController :type "Controller Object Reference"))
  ;[1 1 1] Stop playing animation
  (if (`Controller.IsPlayerController` OldController)
    (`SkeletalMeshComponent.Stop` (`self.Row_R`))
    (`SkeletalMeshComponent.Stop` (`self.Row_L`))))

(event `self.ReceiveTick`
  (params (DeltaSeconds :type "Float (single-precision)"))
  (`parent.ReceiveTick` DeltaSeconds))

(event `self.RowAnimation`
  (params (RowSpeed :type "Float (double-precision)"))
  ;[1 1 1] Row Animation
  (`SkeletalMeshComponent.SetPlayRate` (`self.Row_R`) (* RowSpeed 1.5))
  (`SkeletalMeshComponent.SetPlayRate` (`self.Row_L`) (* RowSpeed 1.5)))

(fn `UserConstructionScript`
  (`parent.UserConstructionScript`))