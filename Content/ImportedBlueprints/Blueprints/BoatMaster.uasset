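; Base pawn for drivable boats, with submarine and hover bike options, rowboat animation hook, boost and position reset.
; Smoothed inputs drive force and torque, while Tick applies a height-restoring force, sway and tilt, plus collision sounds, HUD and camera updates.
; Looped downward traces adjust target height, checking physical material except for hover bikes.
; Player overlap with a sphere toggles ticking and gravity; the exit logic is left unconnected.
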(event OnComponentBeginOverlap(Sphere)
  (params (OverlappedComponent :type Primitive%20Component%20Object%20Reference) (OtherActor :type Actor%20Object%20Reference) (OtherComp :type Primitive%20Component%20Object%20Reference) (OtherBodyIndex :type Integer) (bFromSweep :type Boolean) (SweepResult :type Hit%20Result%20Structure%20%28by%20ref%29))
  ;[1 1 1] Main Logic
  ;;[1 0.5311 0.5411] ACTIVATE PHYSICS IF PLAYER IS NEARBY OR IS POSSESSED BY PLAYER AT THE START (Player should be inside the collision sphere, going outside deactivates ticking and physics)
  (Variables|Don'tTouch|SetReqestedHeight (.z (Transformation|GetWorldLocation (Variables|Default|GetDefaultSceneRoot))))
  (Variables|Don'tTouch|SetReqestedHeight_Memory (Variables|Don'tTouch|GetReqestedHeight))
  (if (== OtherActor (Pawn|GetControlledPawn (Game|GetPlayerController 0)))
    (Physics|SetEnableGravity (Variables|Default|GetBoat_Interior) true)
    (Actor|Tick|SetActorTickEnabled true)
    (CallFunction|ShouldbeSimulating)
    (if (Variables|UserControlled|GetHeight%20Adjust%20Required)
      (CallFunction|KeepReadingLocation))))

(event OnComponentEndOverlap(Sphere)
  (params (OverlappedComponent :type Primitive%20Component%20Object%20Reference) (OtherActor :type Actor%20Object%20Reference) (OtherComp :type Primitive%20Component%20Object%20Reference) (OtherBodyIndex :type Integer))
  ;[1 1 1] Main Logic
  ;;[1 0.5311 0.5411] ACTIVATE PHYSICS IF PLAYER IS NEARBY OR IS POSSESSED BY PLAYER AT THE START (Player should be inside the collision sphere, going outside deactivates ticking and physics)
  (if (== (Pawn|GetControlledPawn (Game|GetPlayerController 0)) OtherActor)
    (Physics|SetEnableGravity (Variables|Default|GetBoat_Interior) false)
    (Actor|Tick|SetActorTickEnabled false)
    (CallFunction|StoppedSimulating)
    (Variables|Don'tTouch|SetIsIn false)))

(event Custom|ShouldBeSimulating
  ;[1 1 1] Main Logic
  ;;[0 1 0.02899] Some Randomness for Sway and Vertical Oscillations
  (bind _newtrack_0 (Timeline|Vibration Play)))

(event Custom|StoppedSimulating
  ;[1 1 1] Main Logic
  ;;[0 1 0.02899] Some Randomness for Sway and Vertical Oscillations
  (bind _newtrack_0 (Timeline|Vibration Stop)))

(event Custom|KeepReadingLocation
  (bind _boat_exterior (Variables|Default|GetBoat_Exterior))
  (bind _returnvalue (Transformation|GetWorldLocation _boat_exterior))
  ;[1 1 1] Main Logic
  ;;[1 1 1] Adjust to water level if Water Physics Material applied
  (if (and (Variables|Don'tTouch|GetIsIn) (not (Variables|UserControlled|GetIs_Submarine)))
    (Utilities|FlowControl|RetriggerableDelay (/ 1e+01 (Variables|UserControlled|GetWaterHeightAdjustResponsiveness)))
    (bind _out_hit_distance (Utilities|ReferenceHeightAdjust (+ (Math|Vector|MakeVector 0.0 0.0 5e+02) _returnvalue) (+ (Math|Vector|MakeVector 0.0 0.0 -1.5e+04) _returnvalue) (Variables|UserControlled|GetHeight%20Adjust%20Required))
      (:True
        (Variables|Don'tTouch|SetAdjustHeightData _out_hit_distance)
        (Variables|Don'tTouch|SetHeightDiff (Math|Interpolation|FInterpTo (Variables|Don'tTouch|GetHeightDiff) (- (Variables|Don'tTouch|GetCurrentAdjustHeightData) (Variables|Don'tTouch|GetAdjustHeightData)) (Utilities|Time|GetWorldDeltaSeconds) 1.0))
        (Variables|Don'tTouch|SetReqestedHeight (+ (Variables|Don'tTouch|GetReqestedHeight) (Variables|Don'tTouch|GetHeightDiff))))
      (:False
        _))
    (CallFunction|KeepReadingLocation)))

(event Custom|RowAnimation
  (params (RowSpeed :type Float%20%28double-precision%29))
  ;[1 1 1] Main Logic
  ;;[0.04597 1 0] Don't Touch. It is used in rowboat templates
)

(event Custom|Entered
  (bind _defaultsceneroot (Variables|Default|GetDefaultSceneRoot))
  (bind _returnvalue (Transformation|GetWorldLocation _defaultsceneroot))
  ;[1 1 1] Main Logic
  ;;[1 0.0191 0 1 28] You must call this function to say that you have entered
  (Class|PrimitiveComponent|SetAllPhysicsLinearVelocity (Variables|Default|GetBoat_Exterior) "0, 0, 0" false)
  (Variables|Don'tTouch|SetVelocity "0, 0, 0")
  (Variables|Don'tTouch|SetPrevVel "0, 0, 0")
  (Variables|Don'tTouch|SetPower 0.0)
  (CallFunction|ShouldbeSimulating)
  (bind _returnvalue_2 (UserInterface|CreateWidget "/Game/ImportedBlueprints/Blueprints/SpeedAndDirection.SpeedAndDirection_C"))
  (bind _output_get (Variables|Don'tTouch|SetAs%20Speed%20HUD _returnvalue_2))
  (UserInterface|Viewport|AddtoViewport _output_get 0)
  ;;[1 1 1] Custom  Enter/Exit logic connect here
  ;;;[1 1 1] After Entering
  (Actor|Tick|SetActorTickEnabled true)
  (Variables|Don'tTouch|SetIsIn true)
  ;;[1 0.8954 0.4689 1 16] Water level, you can define it during spawning according to your game or just placing it at water level should be sufficiemt
  (Variables|Don'tTouch|SetReqestedHeight (.z (Transformation|GetWorldLocation _defaultsceneroot)))
  (bind _out_hit_distance (Utilities|ReferenceHeightAdjust (+ (Math|Vector|MakeVector 0.0 0.0 5e+02) _returnvalue) (+ (Math|Vector|MakeVector 0.0 0.0 -1.5e+04) _returnvalue) (Variables|UserControlled|GetHeight%20Adjust%20Required))
    (:True
      (bind _output_get_2 (Variables|Don'tTouch|SetCurrentAdjustHeightData _out_hit_distance))
      (Variables|Don'tTouch|SetAdjustHeightData _output_get_2))
    (:False
      _))
  ;;[0.01217 1 0.7689] Check if it is controlled by the player
  (if (Class|Controller|IsPlayerController (Pawn|GetController))
    (Variables|Don'tTouch|SetIsIn true)
    (Variables|Don'tTouch|SetReqestedHeight_Memory (Variables|Don'tTouch|GetReqestedHeight))
    ;;[1 0.5311 0.5411] ACTIVATE PHYSICS IF PLAYER IS NEARBY OR IS POSSESSED BY PLAYER AT THE START (Player should be inside the collision sphere, going outside deactivates ticking and physics)
    (Actor|Tick|SetActorTickEnabled true)
    (CallFunction|ShouldbeSimulating)
    (if (Variables|UserControlled|GetHeight%20Adjust%20Required)
      (CallFunction|KeepReadingLocation))))

(event EventBeginPlay
  (bind _defaultsceneroot (Variables|Default|GetDefaultSceneRoot))
  (bind _returnvalue (Transformation|GetWorldLocation _defaultsceneroot))
  ;[1 1 1] Main Logic
  ;;[1 0.8954 0.4689 1 16] Water level, you can define it during spawning according to your game or just placing it at water level should be sufficiemt
  (Utilities|FlowControl|Delay 0.2)
  (Variables|Don'tTouch|SetReqestedHeight (.z (Transformation|GetWorldLocation _defaultsceneroot)))
  (bind _out_hit_distance (Utilities|ReferenceHeightAdjust (+ (Math|Vector|MakeVector 0.0 0.0 5e+02) _returnvalue) (+ (Math|Vector|MakeVector 0.0 0.0 -1.5e+04) _returnvalue) (Variables|UserControlled|GetHeight%20Adjust%20Required))
    (:True
      (bind _output_get (Variables|Don'tTouch|SetCurrentAdjustHeightData _out_hit_distance))
      (Variables|Don'tTouch|SetAdjustHeightData _output_get))
    (:False
      _))
  ;;[0.01217 1 0.7689] Check if it is controlled by the player
  (if (Class|Controller|IsPlayerController (Pawn|GetController))
    (Variables|Don'tTouch|SetIsIn true)
    (Variables|Don'tTouch|SetReqestedHeight_Memory (Variables|Don'tTouch|GetReqestedHeight))
    ;;[1 0.5311 0.5411] ACTIVATE PHYSICS IF PLAYER IS NEARBY OR IS POSSESSED BY PLAYER AT THE START (Player should be inside the collision sphere, going outside deactivates ticking and physics)
    (Actor|Tick|SetActorTickEnabled true)
    (CallFunction|ShouldbeSimulating)
    (if (Variables|UserControlled|GetHeight%20Adjust%20Required)
      (CallFunction|KeepReadingLocation))))

(event EventPossessed
  (params (NewController :type Controller%20Object%20Reference))
  (bind _defaultsceneroot (Variables|Default|GetDefaultSceneRoot))
  (bind _returnvalue (Transformation|GetWorldLocation _defaultsceneroot))
  ;[1 1 1] Main Logic
  ;;[1 1 1] Custom  Enter/Exit logic connect here
  ;;;[1 1 1] After Entering
  (if (Class|Controller|IsPlayerController NewController)
    (Actor|Tick|SetActorTickEnabled true)
    (Variables|Don'tTouch|SetIsIn true)
    ;;[1 0.8954 0.4689 1 16] Water level, you can define it during spawning according to your game or just placing it at water level should be sufficiemt
    (Variables|Don'tTouch|SetReqestedHeight (.z (Transformation|GetWorldLocation _defaultsceneroot)))
    (bind _out_hit_distance (Utilities|ReferenceHeightAdjust (+ (Math|Vector|MakeVector 0.0 0.0 5e+02) _returnvalue) (+ (Math|Vector|MakeVector 0.0 0.0 -1.5e+04) _returnvalue) (Variables|UserControlled|GetHeight%20Adjust%20Required))
      (:True
        (bind _output_get (Variables|Don'tTouch|SetCurrentAdjustHeightData _out_hit_distance))
        (Variables|Don'tTouch|SetAdjustHeightData _output_get))
      (:False
        _))
    ;;[0.01217 1 0.7689] Check if it is controlled by the player
    (if (Class|Controller|IsPlayerController (Pawn|GetController))
      (Variables|Don'tTouch|SetIsIn true)
      (Variables|Don'tTouch|SetReqestedHeight_Memory (Variables|Don'tTouch|GetReqestedHeight))
      ;;[1 0.5311 0.5411] ACTIVATE PHYSICS IF PLAYER IS NEARBY OR IS POSSESSED BY PLAYER AT THE START (Player should be inside the collision sphere, going outside deactivates ticking and physics)
      (Actor|Tick|SetActorTickEnabled true)
      (CallFunction|ShouldbeSimulating)
      (if (Variables|UserControlled|GetHeight%20Adjust%20Required)
        (CallFunction|KeepReadingLocation)))))

(event EventTick
  (params (DeltaSeconds :type Float%20%28single-precision%29))
  (bind _camera (Variables|Default|GetCamera))
  (bind _sway_amount (Variables|UserControlled|GetSway%20amount))
  (bind _power (Variables|Don'tTouch|GetPower))
  (bind _boat_exterior (Variables|Default|GetBoat_Exterior))
  (bind _as_speed_hud (Variables|Don'tTouch|GetAs%20Speed%20HUD))
  (bind _returnvalue (Math|Float|Absolute(Float) _power))
  (bind _returnvalue_2 (Transformation|GetRelativeTransform _camera))
  ;[1 1 1] Main Logic
  ;;[1 0.03818 0] Restoring Z Force
  (Physics|AddForce (Variables|Default|GetBoat_Exterior) (Math|Vector|MakeVector 0.0 0.0 (+ (* (stale Custom|ShouldBeSimulating _newtrack_0) 8e+01) (.z (Math|Conversions|ToVector(Float) (* (- (Variables|Don'tTouch|GetReqestedHeight) (.z (Transformation|GetWorldLocation (Variables|Default|GetBoat_Exterior)))) 155.0))))) "None" true)
  ;;[0.3625 1 0.9502] Random Sway
  (Variables|Don'tTouch|SetSwayVariable (Math|Interpolation|FInterpTo (Variables|Don'tTouch|GetSwayVariable) (stale Custom|ShouldBeSimulating _newtrack_0) (Utilities|Time|GetWorldDeltaSeconds) 0.5))
  (Transformation|SetRelativeRotation _boat_exterior (Math|Rotator|MakeRotator (+ (* _sway_amount (Variables|Don'tTouch|GetSwayVariable)) (* (Variables|Don'tTouch|GetTurnRate) (Variables|UserControlled|GetMaxTilt) (Math|Float|SelectFloat -1.0 1.0 (Variables|UserControlled|GetReverseDirectionOfTilt)) (/ (Math|Vector|VectorLength (Transformation|GetComponentVelocity (Variables|Default|GetBoat_Exterior))) (Variables|UserControlled|GetBoostedForce)) 1.0)) (* _sway_amount (Variables|Don'tTouch|GetSwayVariable)) (.yaw (Transformation|GetWorldRotation _boat_exterior))) true false)
  ;;[0.2474 0.3933 1] Detect Collision Using Acceleration and Play Sound
  (Variables|Don'tTouch|SetVelocity (Transformation|GetComponentVelocity (Variables|Default|GetBoat_Exterior)))
  (if (> (Math|Vector|VectorLength (- (Variables|Don'tTouch|GetPrevVel) (Variables|Don'tTouch|GetVelocity))) (Variables|UserControlled|GetCollision%20Strength%20to%20Trigger%20Sound))
    (Utilities|FlowControl|DoOnce false :!label _label
      (:Completed
        (Utilities|FlowControl|Sequence
          (:then_0
            ;;;[0 1 0.3052] Change Collision Sound Here
            (Audio|PlaySoundatLocation (Variables|UserControlled|GetCollisionSound) (Transformation|GetWorldLocation (Variables|Default|GetBoat_Exterior)) "0, 0, 0" 1.0 1.0 0.0 0 0 0 0))
          (:then_1
            (Utilities|FlowControl|Delay 0.5)
            (goto _label Reset))))))
  ;;[1 0.285 0] Hud Data
  (Variables|Don'tTouch|SetPrevVel (Variables|Don'tTouch|GetVelocity))
  (Utilities|IsValid _as_speed_hud
    (:Is%20Valid
      (Variables|/Game/ImportedBlueprints/Blueprints/SpeedAndDirection.SpeedAndDirection_C|SetSpeedValue _as_speed_hud (Utilities|String|ToString(Text) (Utilities|Text|ToText(String) (Utilities|String|Append (Utilities|String|GetSubstring (Utilities|String|ToString(Float) (* (Math|Vector|VectorLength (Variables|Don'tTouch|GetVelocity)) 0.036)) 0 4) " km/h"))))
      (Variables|/Game/ImportedBlueprints/Blueprints/SpeedAndDirection.SpeedAndDirection_C|SetPower_Value _as_speed_hud _returnvalue)
      (Variables|/Game/ImportedBlueprints/Blueprints/SpeedAndDirection.SpeedAndDirection_C|SetOpacity _as_speed_hud (Utilities|Struct|MakeLinearColor 1.0 1.0 1.0 (* (stale _blink) (Math|Conversions|ToFloat(Integer) (Math|Float|Floor (+ _returnvalue 0.1))))))
      (Default|DirectionChange _as_speed_hud (Math|Float|MapRangeClamped (.yaw (Transformation|GetWorldRotation (Variables|Default|GetArrow))) -1.8e+02 1.8e+02 -0.5 0.5)))
    (:Is%20Not%20Valid
      _))
  ;;[1 1 1] SetCameraRotation
  (Transformation|AddRelativeRotation _camera (Math|Rotator|MakeRotator 0.0 (Class|Actor|GetInputAxisKeyValue) (Class|Actor|GetInputAxisKeyValue)) false false)
  (if (or (< (.pitch (.rotation _returnvalue_2)) -6e+01) (> (.pitch (.rotation _returnvalue_2)) 6e+01))
    (Transformation|SetRelativeRotation (Variables|Default|GetCamera) (Math|Rotator|MakeRotator (.roll (.rotation _returnvalue_2)) (Math|Float|SelectFloat -6e+01 6e+01 (< (.pitch (.rotation _returnvalue_2)) 0.0)) (.yaw (.rotation _returnvalue_2))) false false))
  ;;[1 1 1] Submarine UP/DOWN controls
  (if (Variables|UserControlled|GetIs_Submarine)
    (if (not (and (> (.z (Transformation|GetWorldLocation (Variables|Default|GetBoat_Exterior))) (Variables|Don'tTouch|GetReqestedHeight_Memory)) (> (Variables|Don'tTouch|GetUp/Down_Delta) 0.0)))
      (Variables|Don'tTouch|SetReqestedHeight (+ (* (Variables|Don'tTouch|GetUp/Down_Delta) (Variables|UserControlled|Getup/down_Velocity)) (Variables|Don'tTouch|GetReqestedHeight))))))

(event Input|ActionEvents|InputActionBoost
  (params (Key :type Key%20Structure :default "None"))
  ;[1 1 1] Main Logic
  ;;[0.1165 1 0.4432] Controls
  ;;;[1 0.04149 0] Boost_Just for fun
  (:Pressed
    (Variables|Don'tTouch|SetForce_Mem (Variables|UserControlled|GetForce))
    (Variables|UserControlled|SetForce (Variables|UserControlled|GetBoostedForce)))
  (:Released
    (Variables|UserControlled|SetForce (Variables|Don'tTouch|GetForce_Mem))))

(event Input|AxisEvents|InputAxisMoveForward/Backward
  (params (AxisValue :type Float%20%28single-precision%29))
  ;[1 1 1] Main Logic
  ;;[0.1165 1 0.4432] Controls
  (CallFunction|DelayinPower AxisValue)
  (bind _output_get (Variables|Don'tTouch|SetRowSpeed (Math|Interpolation|FInterpTo (Variables|Don'tTouch|GetRowSpeed) 0.0 (Utilities|Time|GetWorldDeltaSeconds) 0.8)))
  (CallFunction|RowAnimation _output_get))

(event Input|AxisEvents|InputAxisMoveRight/Left
  (params (AxisValue :type Float%20%28single-precision%29))
  (bind _power (Variables|Don'tTouch|GetPower))
  ;[1 1 1] Main Logic
  ;;[0.1165 1 0.4432] Controls
  (CallFunction|DelayedTurn (* AxisValue (Math|Float|SelectFloat 1.0 -1.0 (>= _power 0.0)) _power)))

(event Input|KeyboardEvents|F
  (params (Key :type Key%20Structure :default "None"))
  ;[1 1 1] Main Logic
  ;;[1 1 1] Exit Logic
  (:Pressed
    (Variables|Don'tTouch|SetPlayerController (Game|GetPlayerController 0))))

(event Input|KeyboardEvents|R
  (params (Key :type Key%20Structure :default "None"))
  (bind _boat_exterior (Variables|Default|GetBoat_Exterior))
  (bind _reqestedheight_memory (Variables|Don'tTouch|GetReqestedHeight_Memory))
  (bind _returnvalue (Transformation|GetWorldLocation _boat_exterior))
  ;[1 1 1] Main Logic
  ;;[1 1 1] Reset Position is stuck or weird rotation
  (:Pressed
    (Transformation|SetWorldRotation _boat_exterior (Math|Rotator|MakeRotator 0.0 0.0 (.yaw (Transformation|GetWorldRotation _boat_exterior))) true true)
    (Variables|Don'tTouch|SetReqestedHeight _reqestedheight_memory)
    (Transformation|SetWorldLocation _boat_exterior (Math|Vector|MakeVector (.x _returnvalue) (.y _returnvalue) _reqestedheight_memory) true true)))

(event Input|KeyboardEvents|E
  (params (Key :type Key%20Structure :default "None"))
  ;[1 1 1] Main Logic
  ;;[1 1 1] Submarine UP/DOWN controls
  (:Pressed
    (Variables|Don'tTouch|SetUp/Down_Delta -1.0))
  (:Released
    (Variables|Don'tTouch|SetUp/Down_Delta 0.0)))

(event Input|KeyboardEvents|Q
  (params (Key :type Key%20Structure :default "None"))
  ;[1 1 1] Main Logic
  ;;[1 1 1] Submarine UP/DOWN controls
  (:Pressed
    (Variables|Don'tTouch|SetUp/Down_Delta 1.0))
  (:Released
    (Variables|Don'tTouch|SetUp/Down_Delta 0.0)))

(fn ConstructionScript)

(fn DelayinPower
  (params (Power :type Float%20%28double-precision%29))
  (bind _arrow (Variables|Default|GetArrow))
  (bind _returnvalue (Math|Vector|GetForwardVector _arrow))
  ;[0.2584 1 0.636] BOAT TORQUE FUNCTION WITH SOME DELAY TO SIMULATE VISCOUS LIQUID
  (Variables|Don'tTouch|SetPower (Math|Interpolation|FInterpTo (Variables|Don'tTouch|GetPower) Power (Utilities|Time|GetWorldDeltaSeconds) (Variables|UserControlled|GetThrottle%20Responsiveness)))
  (Physics|AddForce (Variables|Default|GetBoat_Exterior) (Math|Vector|MakeVector (* (Math|Vector|DotProduct _returnvalue "1.000000, 0, 0") (* (Variables|Don'tTouch|GetPower) (Variables|UserControlled|GetForce))) (* (Math|Vector|DotProduct _returnvalue "0.000000,1.000000, 0") (* (Variables|Don'tTouch|GetPower) (Variables|UserControlled|GetForce))) 0.0) "None" true))

(fn DelayedTurn
  (params (TurnRate :type Float%20%28double-precision%29))
  ;[0.2584 1 0.636] BOAT TURNING FUNCTION WITH SOME DELAY TO SIMULATE VISCOUS LIQUID
  (Variables|Don'tTouch|SetTurnRate (Math|Interpolation|FInterpTo (Variables|Don'tTouch|GetTurnRate) TurnRate (Utilities|Time|GetWorldDeltaSeconds) (Variables|UserControlled|GetTurn%20Responsiveness)))
  (Class|PrimitiveComponent|AddTorqueinRadians (Variables|Default|GetBoat_Exterior) (Math|Vector|MakeVector 0.0 0.0 (* (Variables|Don'tTouch|GetTurnRate) (Variables|UserControlled|GetUserControlledRotationStrength))) "None" true))